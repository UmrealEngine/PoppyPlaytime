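; BP_TopCat2 is an ending actor that stages a cat's death and then shows the ending screen.
; While IsVis is true, Tick reveals the skeletal mesh after a delay, starts a looping death animation once, and arms overlap through NION.
; An armed overlap shows hand VFX, then after a delay plays the death sound alongside temporary fire, and later adds WBP_Ending to the viewport.
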(event `self.ReceiveActorBeginOverlap`
  (params (OtherActor :type "Actor Object Reference"))
  (if (`self.NION`)
    (`SceneComponent.SetVisibility` (`self.N_HandVFX1`) true false)
    (`KismetSystemLibrary.Delay` 5.0)
    (`|ExecutionSequence`
      (:`then_0`
        (`SceneComponent.SetVisibility` (`self.fire`) true false)
        (`KismetSystemLibrary.Delay` 10.0)
        (`SceneComponent.SetVisibility` (`self.fire`) false false)
        (`KismetSystemLibrary.Delay` 10.0)
        (bind _returnvalue (`|CreateWidget` "/Game/Project/UI/WBP_Ending.WBP_Ending_C"))
        (`UserWidget.AddToViewport` _returnvalue 3))
      (:`then_1`
        (`GameplayStatics.PlaySoundAtLocation` "/Game/Project/JSH/Audio/Catnapdeath.Catnapdeath" (`self.K2_GetActorLocation`) (struct) 1.0 1.0 0.0 null null null null)))))

(event `self.ReceiveTick`
  (params (DeltaSeconds :type "Float (single-precision)"))
  (if (`self.isVis`)
    (`KismetSystemLibrary.Delay` 2.0)
    (`SceneComponent.SetVisibility` (`self.SkeletalMesh`) true false)
    (`|ExecutionSequence`
      (:`then_0`
        (if (not (`self.isAnim`))
          (`SkeletalMeshComponent.PlayAnimation` (`self.SkeletalMesh`) "/Game/Project/JSH/Asset/4/source/Armature_A_NappyCat_NappyCatDeath.Armature_A_NappyCat_NappyCatDeath" true)
          (set `self.isAnim` true)))
      (:`then_1`
        (set `self.NION` true)))))

(fn `UserConstructionScript`)