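; BP_AttackCatNab5 is an actor, apparently for a CatNap attack, that handles the player death presentation through two flags checked on Tick.
; WidgetPlay works as a one-shot trigger that adds one of four randomly picked player death widgets to the viewport.
; While HandDel is set, it hides BP_PoppyPlayer's hands and arm mesh every frame by disabling their main and depth pass rendering.
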(event `self.ReceiveBeginPlay`)

(event `self.ReceiveTick`
  (params (DeltaSeconds :type "Float (single-precision)"))
  (`|ExecutionSequence`
    (:`then_0`
      (if (`self.WidgetPlay`)
        (set `self.WidgetPlay` false)
        (switch `int` (`KismetMathLibrary.RandomInteger` 4)
          (:`Default`
            (bind _returnvalue (`|CreateWidget` "/Game/Project/UI/WBP_PlayerDie1.WBP_PlayerDie1_C" :!label _label))
            (`UserWidget.AddToViewport` _returnvalue 3))
          (:`0`
            (bind _returnvalue_2 (`|CreateWidget` "/Game/Project/UI/WBP_PlayerDie.WBP_PlayerDie_C"))
            (`UserWidget.AddToViewport` _returnvalue_2 3))
          (:`1`
            (goto _label))
          (:`2`
            (bind _returnvalue_3 (`|CreateWidget` "/Game/Project/UI/WBP_PlayerDie2.WBP_PlayerDie2_C"))
            (`UserWidget.AddToViewport` _returnvalue_3 3))
          (:`3`
            (bind _returnvalue_4 (`|CreateWidget` "/Game/Project/UI/WBP_PlayerDie3.WBP_PlayerDie3_C"))
            (`UserWidget.AddToViewport` _returnvalue_4 3)))))
    (:`then_1`
      (bind _asbp_poppy_player (cast `/Game/Project/KMK/BluePrint/BP_PoppyPlayer` (`GameplayStatics.GetPlayerPawn` 0)))
      (bind _output_get (set `KMK_Player.Hands` (`KMK_Player.Hands` _asbp_poppy_player) _asbp_poppy_player))
      (for (_array_element _array_index) _output_get
        (if (`self.HandDel`)
          (`|ExecutionSequence`
            (:`then_0`
              (switch `int` _array_index
                (:`Default`
                  _)
                (:`0`
                  _)
                (:`1`
                  _))
              (bind _output_get_2 (set `KMK_PlayerHand.hand` (`KMK_PlayerHand.hand` _array_element) _array_element))
              (`PrimitiveComponent.SetRenderInMainPass` _output_get_2 false)
              (`PrimitiveComponent.SetRenderInDepthPass` _output_get_2 false))
            (:`then_1`
              (bind _armmesh (`KMK_Player.armMesh` _asbp_poppy_player))
              (`PrimitiveComponent.SetRenderInMainPass` _armmesh false)
              (`PrimitiveComponent.SetRenderInDepthPass` _armmesh false))))))))

(fn `UserConstructionScript`)