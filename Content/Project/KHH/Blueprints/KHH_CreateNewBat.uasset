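; KHH_CreateNewBat is a spawner actor that launches a KHH_NewBat toward the player once, shortly after play begins.
; After a short delay, it spawns the bat at its NewBat component's location, using the player pawn's rotation.
; It then sets the bat Box's physics velocity along the direction from the spawner to the player, scaled by Speed, with no later homing.
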(event `self.ReceiveBeginPlay`
  (`KismetSystemLibrary.Delay` 1.8)
  (bind _returnvalue (`|SpawnActorFromClass` "/Game/Project/KHH/Blueprints/KHH_NewBat.KHH_NewBat_C" (`KismetMathLibrary.MakeTransform` (`SceneComponent.K2_GetComponentLocation` (`self.New_Bat`)) (`self.K2_GetActorRotation` (`GameplayStatics.GetPlayerPawn` 0))) "Undefined" "MultiplyWithRoot" null null))
  (`PrimitiveComponent.SetPhysicsLinearVelocity` (`/Game/Project/KHH/Blueprints/KHH_NewBat.Box` _returnvalue) (* (`KismetMathLibrary.GetDirectionUnitVector` (`self.K2_GetActorLocation`) (`self.K2_GetActorLocation` (`GameplayStatics.GetPlayerPawn` 0))) (`self.speed`)) false "None"))

(fn `UserConstructionScript`)