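; Enemy Blueprint that stalks the player and triggers a jump scare on close contact, starting frozen briefly via custom time dilation.
; Tick reads the FSM state: Idle turns it toward the player controller's location after a delay, while other states periodically toggle its audio and check player distance.
; Within range, it disables player input, hides its mesh and collision, and swaps the player's hands for the JumpScare component via render-pass flags.
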(event `self.ReceiveBeginPlay`
  (set `self.CustomTimeDilation` 0.0)
  (`KismetSystemLibrary.Delay` 0.7)
  (set `self.CustomTimeDilation` 1.0))

(event `self.ReceiveTick`
  (params (DeltaSeconds :type "Float (single-precision)"))
  (bind _returnvalue (`GameplayStatics.GetPlayerPawn` 0))
  (bind _mesh (`self.Mesh`))
  (bind _audiocurvesource (`self.AudioCurveSource`))
  (if (`|EnumEquality` (`KHH_EnemyFSM.mState` (`self.fsm`)) "Idle")
    (`KismetSystemLibrary.Delay` 2.8)
    (`self.K2_SetActorRotation` (`KismetMathLibrary.FindLookAtRotation` (`self.K2_GetActorLocation`) (`self.K2_GetActorLocation` (`GameplayStatics.GetPlayerController` 0))))
    (else
      (`|ExecutionSequence`
        (:`then_0`
          (`KismetSystemLibrary.Delay` 10.0)
          (if (`AudioComponent.IsPlaying` _audiocurvesource)
            (`AudioComponent.Stop` _audiocurvesource)
            (else
              (`AudioComponent.Play` _audiocurvesource 0.0))))
        (:`then_1`
          ;[1 1 1] 거리 확인과 메쉬 on/off 기능만 존재
          (bind _asbp_poppy_player (cast `/Game/Project/KMK/BluePrint/BP_PoppyPlayer` _returnvalue))
          (if (< (`KismetMathLibrary.Vector_Distance` (`self.K2_GetActorLocation` _returnvalue) (`self.K2_GetActorLocation`)) 250.0)
            (`AudioComponent.Stop` (`self.AudioCurveSource`))
            (`self.DisableInput` _asbp_poppy_player null)
            (`SceneComponent.SetVisibility` _mesh false false)
            (`PrimitiveComponent.SetCollisionEnabled` _mesh "NoCollision")
            (bind _output_get (set `KMK_Player.Hands` (`KMK_Player.Hands` _asbp_poppy_player) _asbp_poppy_player))
            (for (_array_element _array_index) _output_get
              (switch `int` _array_index
                (:`0`
                  _)
                (:`1`
                  _))
              (bind _output_get_2 (set `KMK_PlayerHand.hand` (`KMK_PlayerHand.hand` _array_element) _array_element))
              (`PrimitiveComponent.SetRenderInMainPass` _output_get_2 false)
              (`PrimitiveComponent.SetRenderInDepthPass` _output_get_2 false)
              (if (`|EnumEquality` (`KHH_EnemyFSM.mState` (`self.fsm`)) "Die")
                (`AudioComponent.Stop` (`self.AudioCurveSource`))))
            (`PrimitiveComponent.SetRenderInMainPass` (`/Game/Project/KMK/BluePrint/BP_PoppyPlayer.JumpScare` _asbp_poppy_player) true)))))))

(fn `UserConstructionScript`)