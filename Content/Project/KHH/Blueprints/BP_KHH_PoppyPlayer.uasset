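; Poppy horror player Blueprint that freezes a pursuing KHH_Enemy while the player looks at it and handles the jumpscare death.
; A pawn sensor stores enemies not tagged "Del".
; Tick combines AI line of sight with a view-direction dot product to toggle that enemy's time dilation and yaw control.
; When JumpScare renders in main pass, Tick sets rotations, plays it, shakes the camera and shows a delayed death widget.
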(event `self.ReceiveActorBeginOverlap`
  (params (OtherActor :type "Actor Object Reference"))
  (bind _askhh_enemy (cast `KHH_Enemy` OtherActor))
  (set `self.Teacher` _askhh_enemy))

(event `self.ReceiveTick`
  (params (DeltaSeconds :type "Float (single-precision)"))
  (bind _enemy (`self.Enemy`))
  (bind _enemy_2 (`self.Enemy`))
  (bind _enemy_3 (`self.Enemy`))
  (`|ExecutionSequence`
    (:`then_0`
      (`/Engine/EditorBlueprintResources/StandardMacros.IsValid` _enemy_2
        (:`Is Valid`
          (if true
            (bind _asaicontroller (cast `AIController` (`self.GetController` _enemy_2)))
            (if (`Controller.LineOfSightTo` _asaicontroller (`GameplayStatics.GetPlayerCharacter` 0) (0.0 0.0 0.0) false)
              (if (> (`KismetMathLibrary.Dot_VectorVector` (`KismetMathLibrary.GetForwardVector` (`self.GetControlRotation`)) (- (`self.K2_GetActorLocation` (`GameplayStatics.GetPlayerPawn` 0)) (`self.K2_GetActorLocation` (`self.Enemy`)))) -0.6)
                (set `Actor.CustomTimeDilation` 1.0 _enemy :!label _label)
                (set `Pawn.bUseControllerRotationYaw` true _enemy)
                (else
                  (set `Actor.CustomTimeDilation` 0.0 _enemy_3)
                  (set `Pawn.bUseControllerRotationYaw` false _enemy_3)))
              (else
                (goto _label)))))))
    (:`then_1`
      (if (`PrimitiveComponent.bRenderInMainPass` (`self.JumpScare`))
        (`self.K2_SetActorRotation` (struct :`Yaw` 180.0))
        (`SceneComponent.K2_SetWorldRotation` (`self.camera`) (struct :`Pitch` 15.0 :`Yaw` 180.0) false false)
        (`SkeletalMeshComponent.Play` (`self.JumpScare`) false)
        (`|ExecutionSequence`
          (:`then_0`
            (`KismetSystemLibrary.Delay` 2.0)
            (bind _returnvalue (`|CreateWidget` "/Game/Project/UI/WBP_PlayerDie1.WBP_PlayerDie1_C"))
            (`UserWidget.AddToViewport` _returnvalue 0))
          (:`then_1`
            (`GameplayStatics.PlayWorldCameraShake` "/Game/Project/KHH/BP_CameraShake.BP_CameraShake_C" (`self.K2_GetActorLocation`) 0.0 500.0)))))))

(event `self.sensor.OnSeePawn`
  (params (Pawn :type "Pawn Object Reference"))
  (bind _askhh_enemy (cast `KHH_Enemy` Pawn))
  (if (not (`self.ActorHasTag` _askhh_enemy "Del"))
    (set `self.Enemy` _askhh_enemy)))

(fn `UserConstructionScript`)