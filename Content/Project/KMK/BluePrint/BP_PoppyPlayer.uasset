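; Player Blueprint for a horror game, adding a look-to-freeze enemy and a jumpscare death.
; Pawn sensing stores the enemy and its FSM; outside Idle, Tick zeroes its time dilation while it has line of sight and sits within the player's view cone.
; When JumpScare renders, Tick drives camera, shake, sound and a random death widget.
; A cheat input toggles forced freezing; BeginPlay hides spotlights in "JSH" levels.
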(event `self.ReceiveBeginPlay`
  (bind _returnvalue (`GameplayStatics.GetCurrentLevelName` true))
  (if (`KismetStringLibrary.Contains` _returnvalue "JSH")
    (`SceneComponent.SetVisibility` (`self.SpotLight1`) false false)
    (`SceneComponent.SetVisibility` (`self.SpotLight`) false false)))

(event `self.sensor.OnSeePawn`
  (params (Pawn :type "Pawn Object Reference"))
  ;[1 1 1] 플레이어 시야에 딜라이트 들어옴
  (bind _askhh_enemy (cast `KHH_Enemy` Pawn))
  (set `self.EFSM` (`self.GetComponentByClass` _askhh_enemy "/Script/CatTeacher.KHH_EnemyFSM"))
  (if (not (`self.ActorHasTag` _askhh_enemy "Del"))
    (set `self.Enemy` _askhh_enemy)))

(event `self.ReceiveActorBeginOverlap`
  (params (OtherActor :type "Actor Object Reference"))
  (bind _askhh_enemy (cast `KHH_Enemy` OtherActor))
  (set `self.Teacher` _askhh_enemy))

(event `self.ReceiveTick`
  (params (DeltaSeconds :type "Float (single-precision)"))
  (bind _enemy (`self.Enemy`))
  (bind _enemy_2 (`self.Enemy`))
  (bind _enemy_3 (`self.Enemy`))
  (if (`self.isCheat1`)
    (set `Actor.CustomTimeDilation` 0.0 _enemy_2)
    (set `Pawn.bUseControllerRotationYaw` false _enemy_2)
    (else
      (`/Engine/EditorBlueprintResources/StandardMacros.IsValid` (`self.EFSM`)
        (:`Is Valid`
          (if (not (`|EnumEquality` (`KHH_EnemyFSM.mState` (`self.EFSM`)) "Idle"))
            (`|ExecutionSequence`
              (:`then_0`
                (`/Engine/EditorBlueprintResources/StandardMacros.IsValid` _enemy_3
                  (:`Is Valid`
                    (if true
                      (bind _asaicontroller (cast `AIController` (`Pawn.GetController` _enemy_3)))
                      (if (`Controller.LineOfSightTo` _asaicontroller (`GameplayStatics.GetPlayerCharacter` 0) (0.0 0.0 0.0) false)
                        (if (> (`KismetMathLibrary.Dot_VectorVector` (`KismetMathLibrary.GetForwardVector` (`Pawn.GetControlRotation`)) (- (`self.K2_GetActorLocation` (`GameplayStatics.GetPlayerPawn` 0)) (`self.K2_GetActorLocation` (`self.Enemy`)))) -0.6)
                          (set `Actor.CustomTimeDilation` 1.0 _enemy :!label _label)
                          (set `Pawn.bUseControllerRotationYaw` true _enemy)
                          (else
                            (set `Actor.CustomTimeDilation` 0.0 _enemy)
                            (set `Pawn.bUseControllerRotationYaw` false _enemy)))
                        (else
                          (goto _label)))))))
              (:`then_1`
                (if (`self.isEgg`)
                  _
                  (elif (`PrimitiveComponent.bRenderInMainPass` (`self.JumpScare`))
                    (`self.K2_SetActorRotation` (struct :`Yaw` 180.0))
                    ;[0.07573 1 0.2293] CameraShake
                    (if (`self.JumpScareStart`)
                      (`SceneComponent.K2_SetWorldRotation` (`self.camera`) (struct :`Pitch` 15.0 :`Yaw` 100.0) false false)
                      (set `self.JumpScareStart` false)
                      (if (not (`self.isRemove`))
                        (`WidgetLayoutLibrary.RemoveAllWidgets`)
                        (set `self.isRemove` true))
                      (`SkeletalMeshComponent.Play` (`self.JumpScare`) false)
                      ;[0.07573 1 0.2293] CameraShake
                      (`GameplayStatics.PlayWorldCameraShake` "/Game/Project/KHH/Blueprints/BP_KHH_CameraShake.BP_KHH_CameraShake_C" (`self.K2_GetActorLocation` (`GameplayStatics.GetPlayerPawn` 0)) 1.0 75.0)
                      (if (not (`self.isSound`))
                        (`GameplayStatics.PlaySound2D` "/Game/Project/KMK/Audio/SW_Teacher_Jumpscare.SW_Teacher_Jumpscare" 1.0 1.0 0.0 null null)
                        (set `self.isSound` true)
                        (`KismetSystemLibrary.Delay` 0.7)
                        (if (not (`self.isWidgeet`))
                          (set `self.isWidgeet` true)
                          (switch `int` (`KismetMathLibrary.RandomInteger` 4)
                            (:`Default`
                              (bind _returnvalue (`|CreateWidget` "/Game/Project/UI/WBP_PlayerDie1.WBP_PlayerDie1_C" :!label _label_2))
                              (`UserWidget.AddToViewport` _returnvalue 3))
                            (:`0`
                              (bind _returnvalue_2 (`|CreateWidget` "/Game/Project/UI/WBP_PlayerDie.WBP_PlayerDie_C"))
                              (`UserWidget.AddToViewport` _returnvalue_2 3))
                            (:`1`
                              (goto _label_2))
                            (:`2`
                              (bind _returnvalue_3 (`|CreateWidget` "/Game/Project/UI/WBP_PlayerDie2.WBP_PlayerDie2_C"))
                              (`UserWidget.AddToViewport` _returnvalue_3 3))
                            (:`3`
                              (bind _returnvalue_4 (`|CreateWidget` "/Game/Project/UI/WBP_PlayerDie3.WBP_PlayerDie3_C"))
                              (`UserWidget.AddToViewport` _returnvalue_4 3))))))))))))))))

(event `EnhancedInput|/Game/Project/KMK/Controller/MIA/MIA_Cheater1`
  (params (ActionValue :type Boolean) (ElapsedSeconds :type "Float (double-precision)") (TriggeredSeconds :type "Float (double-precision)") (InputAction :type "InputAction Object Reference" :default "/Game/Project/KMK/Controller/MIA/MIA_Cheater1.MIA_Cheater1"))
  (:`Started`
    (set `self.isCheat1` (not (`self.isCheat1`)))))

(fn `UserConstructionScript`)